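; EndStartBase shows either the start screen or the end screen when play begins, based on the game state.
; On BeginPlay it reads MyCurrentState from MyGameInstance and creates StartScreen for the first state, or EndScreen plus Leaderboard for any other.
; Both paths show the mouse cursor.
; The end path then looks up Leaderboard widgets by class and calls UpdateLeaderboard on them.
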(event `self.ReceiveBeginPlay`
  (bind _asmy_game_instance (cast `/Game/MyGameInstance` (`GameplayStatics.GetGameInstance`)))
  (if (`|EnumEquality` (`/Game/MyGameInstance.MyCurrentState` _asmy_game_instance) "NewEnumerator0")
    (bind _returnvalue (`|CreateWidget` "/Game/UI/StartScreen.StartScreen_C"))
    (`UserWidget.AddToViewport` _returnvalue 0)
    (set `PlayerController.bShowMouseCursor` true (`GameplayStatics.GetPlayerController` 0))
    (else
      (bind _returnvalue_2 (`|CreateWidget` "/Game/UI/EndScreen.EndScreen_C"))
      (`UserWidget.AddToViewport` _returnvalue_2 0)
      (set `PlayerController.bShowMouseCursor` true (`GameplayStatics.GetPlayerController` 0))
      (bind _returnvalue_3 (`|CreateWidget` "/Game/UI/Leaderboard.Leaderboard_C"))
      (`UserWidget.AddToViewport` _returnvalue_3 0)
      (bind _foundwidgets (`WidgetBlueprintLibrary.GetAllWidgetsOfClass` "/Game/UI/Leaderboard.Leaderboard_C" false))
      (`/Game/UI/Leaderboard.Update Leaderboard` _foundwidgets))))

(fn `UserConstructionScript`)