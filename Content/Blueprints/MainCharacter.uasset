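; Player character for a shooter, handling health, respawning, pause menu and input sound effects.
; BeginPlay caches spawn points and creates hidden leaderboard and pause widgets, which Escape toggles along with game pause and cursor.
; Overlaps with two bullet types subtract health and record the shooter, while Health pickups heal.
; Tick caps health and refreshes its UI; at zero it teleports to a random spawn and passes the last shooter to the GameInstance.
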(event `Key|LeftMouseButton`
  (params (Key :type "Key Structure"))
  (:`Pressed`
    (`GameplayStatics.PlaySound2D` "/Game/Audio/laser-shot-ingame-230500.laser-shot-ingame-230500" 1.0 1.0 0.0 null null)))

(event `Key|SpaceBar`
  (params (Key :type "Key Structure"))
  (:`Pressed`
    (`GameplayStatics.PlaySound2D` "/Game/Audio/sfx_jump_07-80241.sfx_jump_07-80241" 1.0 1.0 0.0 null null)))

(event `Key|Escape` :paused true
  (params (Key :type "Key Structure"))
  (bind _leaderboardpause (`self.LeaderboardPause`))
  (:`Pressed`
    (if (`self.leaderboard Display`)
      (`Widget.SetVisibility` _leaderboardpause "Collapsed")
      (`Widget.SetVisibility` (`self.PauseButtons`) "Collapsed")
      (set `self.leaderboard Display` false)
      (`GameplayStatics.SetGamePaused` false)
      (set `PlayerController.bShowMouseCursor` false (`GameplayStatics.GetPlayerController` 0))
      (else
        (`Widget.SetVisibility` _leaderboardpause "Visible")
        (`Widget.SetVisibility` (`self.PauseButtons`) "Visible")
        (set `self.leaderboard Display` true)
        (`GameplayStatics.SetGamePaused` true)
        (set `PlayerController.bShowMouseCursor` true (`GameplayStatics.GetPlayerController` 0))))))

(event `self.ReceiveBeginPlay`
  (bind _outactors (`GameplayStatics.GetAllActorsOfClass` "/Game/Blueprints/CharacterSpawnPoint.CharacterSpawnPoint_C"))
  (set `self.Out Actors` _outactors)
  (bind _returnvalue (`|CreateWidget` "/Game/UI/Leaderboard.Leaderboard_C"))
  (bind _output_get (set `self.LeaderboardPause` _returnvalue))
  (`UserWidget.AddToViewport` _returnvalue 0)
  (`UserWidget.AddToViewport` _output_get 0)
  (`Widget.SetVisibility` _output_get "Collapsed")
  (bind _returnvalue_2 (`|CreateWidget` "/Game/UI/PausedGame.PausedGame_C"))
  (bind _output_get_2 (set `self.PauseButtons` _returnvalue_2))
  (`UserWidget.AddToViewport` _output_get_2 0)
  (`Widget.SetVisibility` _returnvalue_2 "Collapsed"))

(event `self.ReceiveActorBeginOverlap`
  (params (OtherActor :type "Actor Object Reference"))
  (bind _asbullets_for_gun (cast `/Game/Blueprints/BulletsForGun` OtherActor)
    (:`then`
      (bind _output_get (set `BulletProjectile.ShooterName` (`BulletProjectile.ShooterName` _asbullets_for_gun) _asbullets_for_gun))
      (set `self.LastPersonShot` _output_get)
      (set `self.MainCharacterHealth` (+ (`self.MainCharacterHealth`) -3)))
    (:`CastFailed`
      (bind _asbullets_for_gun_2 (cast `/Game/Blueprints/BulletsForGun2` OtherActor)
        (:`then`
          (bind _output_get_2 (set `BulletProjectile.ShooterName` (`BulletProjectile.ShooterName` _asbullets_for_gun_2) _asbullets_for_gun_2))
          (set `self.LastPersonShot` _output_get_2)
          (set `self.MainCharacterHealth` (+ (`self.MainCharacterHealth`) -12)))
        (:`CastFailed`
          (cast `/Game/Blueprints/Health` OtherActor)
          (set `self.MainCharacterHealth` (+ (`self.MainCharacterHealth`) 25))
          (`self.UpdateHealthUi`))))))

(event `self.ReceiveTick`
  (params (DeltaSeconds :type "Float (single-precision)"))
  (if (<= (`self.MainCharacterHealth`) 0)
    (`self.K2_TeleportTo` :`self` self :`DestLocation` (`self.K2_GetActorLocation` (`KismetArrayLibrary.Array_Random` (`self.Out Actors`))))
    (set `self.MainCharacterHealth` 100)
    (`self.UpdateHealthUi`)
    (`self.onKilledConfirmed` (`self.LastPersonShot`))
    (`GameplayStatics.PlaySound2D` "/Game/Audio/game-over-arcade-6435.game-over-arcade-6435" 1.0 1.0 0.0 null null)
    (elif (> (`self.MainCharacterHealth`) 100)
      (set `self.MainCharacterHealth` 100)
      (`self.UpdateHealthUi`)
      (else
        (`self.UpdateHealthUi`)))))

(event `/Game/Blueprints/KillTrackerInterface.onKilledConfirmed`
  (params (KillerName :type String))
  (bind _asmy_game_instance (cast `/Game/MyGameInstance` (`GameplayStatics.GetGameInstance`)))
  (`/Game/MyGameInstance.AddPlayerData` _asmy_game_instance KillerName 0))

(fn `UserConstructionScript`)