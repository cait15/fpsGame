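; BP_TheAI is a combat bot that fights the player and other bots, feeding its state to a Blackboard.
; Pawn sensing triggers attacks with either of two guns based on secondary ammo, or flight at low health.
; AI perception flags health or ammo pickups, and overlaps apply bullet damage and pickups.
; On death it teleports to a random spawn point, resets health and reports the last shooter to the game instance.
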(event `self.ReceiveTick`
  (params (DeltaSeconds :type "Float (single-precision)"))
  (`BlackboardComponent.SetValueAsInt` (`AIBlueprintHelperLibrary.GetBlackboard` (`AIBlueprintHelperLibrary.GetAIController` self)) "AiHealth" (`self.AIHealth`))
  (if (<= (`self.AIHealth`) 0)
    (`self.K2_TeleportTo` (`self.K2_GetActorLocation` (`KismetArrayLibrary.Array_Random` (`self.Out Actors`))))
    (`self.onKilledConfirmed` (`self.LastPersonShotName`))
    (set `self.AIHealth` 100)
    (`BlackboardComponent.SetValueAsBool` (`AIBlueprintHelperLibrary.GetBlackboard` (`AIBlueprintHelperLibrary.GetAIController` self)) "RoamAround" false)
    (else
      (if (== (`self.Secondaryammo`) 0)
        (set `self.Weapon 2Unlocked` false)
        (else
          (set `self.Weapon 2Unlocked` true)))
      (if (>= (`self.AIHealth`) 100)
        (set `self.AIHealth` 100)))))

(event `self.ReceiveActorBeginOverlap`
  (params (OtherActor :type "Actor Object Reference"))
  (bind _asbullets_for_gun (cast `/Game/Blueprints/BulletsForGun` OtherActor)
    (:`then`
      (bind _output_get (set `BulletProjectile.ShooterName` (`BulletProjectile.ShooterName` _asbullets_for_gun) _asbullets_for_gun))
      (set `self.LastPersonShotName` _output_get)
      (bind _output_get_2 (set `self.AIHealth` (- (`self.AIHealth`) 3))))
    (:`CastFailed`
      (bind _asbullets_for_gun_2 (cast `/Game/Blueprints/BulletsForGun2` OtherActor)
        (:`then`
          (bind _output_get_3 (set `BulletProjectile.ShooterName` (`BulletProjectile.ShooterName` _asbullets_for_gun_2) _asbullets_for_gun_2))
          (set `self.LastPersonShotName` _output_get_3)
          (bind _output_get_4 (set `self.AIHealth` (- (`self.AIHealth`) 12))))
        (:`CastFailed`
          (cast `/Game/MyPickUpBase` OtherActor
            (:`then`
              (bind _output_get_5 (set `self.Secondaryammo` 10))
              (`KismetSystemLibrary.PrintString` (`KismetStringLibrary.Conv_IntToString` _output_get_5))
              (set `self.Weapon 2Unlocked` true)
              (`self.ReloadGun2`))
            (:`CastFailed`
              (cast `/Game/Blueprints/Health` OtherActor)
              (set `self.AIHealth` (+ (`self.AiHealth`) 25))
              (`KismetSystemLibrary.PrintString` "Hello")
              (if (> (`self.AIHealth`) 100)
                (set `self.AiHealth` 100)))))))))

(event `self.ReceiveBeginPlay`
  (`self.SetOwner` (`ChildActorComponent.ChildActor` (`self.PrimaryWeapon`)) self)
  (`self.SetOwner` (`ChildActorComponent.ChildActor` (`self.SecondaryWeapon`)) self)
  (`SceneComponent.ToggleVisibility` (`self.PrimaryWeapon`) false)
  (`SceneComponent.K2_AttachToComponent` (`self.SecondaryWeapon`) (`self.Mesh`) "GripPoint" "KeepRelative" "KeepRelative" "KeepRelative" true)
  (set `self.Weapon One Attachment` false)
  (set `self.Weapon Two Attachment` true)
  (bind _outactors (`GameplayStatics.GetAllActorsOfClass` "/Game/Blueprints/EnemySpawnPoints.EnemySpawnPoints_C"))
  (set `self.Out Actors` _outactors)
  (`BlackboardComponent.SetValueAsBool` (`AIBlueprintHelperLibrary.GetBlackboard` (`AIBlueprintHelperLibrary.GetAIController` self)) "RoamAround" true))

(event `self.PawnSensing.OnSeePawn`
  (params (Pawn :type "Pawn Object Reference"))
  (if (> (`self.AIHealth`) 25)
    (cast `/Game/Blueprints/MainCharacter` Pawn
      (:`then`
        (`BlackboardComponent.SetValueAsBool` (`AIBlueprintHelperLibrary.GetBlackboard` (`AIBlueprintHelperLibrary.GetAIController` self)) "IsPlayerTarget?" true)
        (`BlackboardComponent.SetValueAsBool` (`AIBlueprintHelperLibrary.GetBlackboard` (`AIBlueprintHelperLibrary.GetAIController` self)) "RoamAround" false)
        (`BlackboardComponent.SetValueAsBool` (`AIBlueprintHelperLibrary.GetBlackboard` (`AIBlueprintHelperLibrary.GetAIController` self)) "RunAway" false)
        (`BlackboardComponent.SetValueAsBool` (`AIBlueprintHelperLibrary.GetBlackboard` (`AIBlueprintHelperLibrary.GetAIController` self)) "Attacking" true)
        (if (`self.Weapon 2Unlocked`)
          (if (== (`self.Secondaryammo`) 0)
            (if (`self.Weapon One Attachment`) :!label _label
              (`self.FireGun1`)
              (else
                (`SceneComponent.ToggleVisibility` (`self.PrimaryWeapon`) false)
                (`SceneComponent.K2_AttachToComponent` (`self.PrimaryWeapon`) (`self.Mesh`) "GripPoint" "KeepRelative" "KeepRelative" "KeepRelative" true)
                (`SceneComponent.ToggleVisibility` (`self.SecondaryWeapon`) false)
                (set `self.Weapon One Attachment` true)
                (set `self.Weapon Two Attachment` false)
                (`KismetSystemLibrary.Delay` 5.0)
                (`self.FireGun1`)))
            (elif (`self.Weapon Two Attachment`)
              (`self.FireGun2`)
              (else
                (`SceneComponent.ToggleVisibility` (`self.SecondaryWeapon`) false)
                (`SceneComponent.K2_AttachToComponent` (`self.SecondaryWeapon`) (`self.Mesh`) "GripPoint" "KeepRelative" "KeepRelative" "KeepRelative" true)
                (`SceneComponent.ToggleVisibility` (`self.PrimaryWeapon`) false)
                (set `self.Weapon Two Attachment` true)
                (set `self.Weapon One Attachment` false)
                (`self.FireGun2`))))
          (else
            (goto _label))))
      (:`CastFailed`
        (cast `/Game/Blueprints/FixingAI/BP/BP_TheAI` Pawn)
        (`BlackboardComponent.SetValueAsBool` (`AIBlueprintHelperLibrary.GetBlackboard` (`AIBlueprintHelperLibrary.GetAIController` self)) "IsPlayerTarget?" false)
        (`BlackboardComponent.SetValueAsBool` (`AIBlueprintHelperLibrary.GetBlackboard` (`AIBlueprintHelperLibrary.GetAIController` self)) "RoamAround" false)
        (`BlackboardComponent.SetValueAsBool` (`AIBlueprintHelperLibrary.GetBlackboard` (`AIBlueprintHelperLibrary.GetAIController` self)) "RunAway" false)
        (`BlackboardComponent.SetValueAsBool` (`AIBlueprintHelperLibrary.GetBlackboard` (`AIBlueprintHelperLibrary.GetAIController` self)) "Attacking" true)
        (`BlackboardComponent.SetValueAsObject` (`AIBlueprintHelperLibrary.GetBlackboard` (`AIBlueprintHelperLibrary.GetAIController` self)) "FoundTarget" Pawn)
        (if true
          (if (== (`self.Secondaryammo`) 0)
            (if (`self.Weapon One Attachment`) :!label _label_2
              (`self.FireGun1`)
              (else
                (`SceneComponent.ToggleVisibility` (`self.PrimaryWeapon`) false)
                (`SceneComponent.K2_AttachToComponent` (`self.PrimaryWeapon`) (`self.Mesh`) "GripPoint" "KeepRelative" "KeepRelative" "KeepRelative" true)
                (`SceneComponent.ToggleVisibility` (`self.SecondaryWeapon`) false)
                (set `self.Weapon One Attachment` true)
                (set `self.Weapon Two Attachment` false)
                (`KismetSystemLibrary.Delay` 5.0)
                (`self.FireGun1`)))
            (elif (`self.Weapon Two Attachment`)
              (`self.FireGun2`)
              (else
                (`SceneComponent.ToggleVisibility` (`self.SecondaryWeapon`) false)
                (`SceneComponent.K2_AttachToComponent` (`self.SecondaryWeapon`) (`self.Mesh`) "GripPoint" "KeepRelative" "KeepRelative" "KeepRelative" true)
                (`SceneComponent.ToggleVisibility` (`self.PrimaryWeapon`) false)
                (set `self.Weapon Two Attachment` true)
                (set `self.Weapon One Attachment` false)
                (`self.FireGun2`))))
          (else
            (goto _label_2)))))
    (else
      (`BlackboardComponent.SetValueAsBool` (`AIBlueprintHelperLibrary.GetBlackboard` (`AIBlueprintHelperLibrary.GetAIController` self)) "RunAway" true)
      (`BlackboardComponent.SetValueAsBool` (`AIBlueprintHelperLibrary.GetBlackboard` (`AIBlueprintHelperLibrary.GetAIController` self)) "Attacking" false)
      (`BlackboardComponent.SetValueAsBool` (`AIBlueprintHelperLibrary.GetBlackboard` (`AIBlueprintHelperLibrary.GetAIController` self)) "RoamAround" false)
      (if (== (`BlackboardComponent.GetValueAsBool` (`AIBlueprintHelperLibrary.GetBlackboard` (`AIBlueprintHelperLibrary.GetAIController` self)) "IsPickUpInReach?") true)
        (`BlackboardComponent.SetValueAsBool` (`AIBlueprintHelperLibrary.GetBlackboard` (`AIBlueprintHelperLibrary.GetAIController` self)) "Fleeing" false)
        (else
          (`BlackboardComponent.SetValueAsBool` (`AIBlueprintHelperLibrary.GetBlackboard` (`AIBlueprintHelperLibrary.GetAIController` self)) "Fleeing" true))))))

(event `FireGun2`
  (bind _assecondarytestgun (cast `/Game/Blueprints/SECONDARYTESTGUN` (`ChildActorComponent.ChildActor` (`self.SecondaryWeapon`))))
  (`KismetSystemLibrary.Delay` 0.5)
  (`GunBase.Fire` _assecondarytestgun)
  (bind _result (`/Engine/EditorBlueprintResources/StandardMacros.DecrementInt` (`self.Secondaryammo`))
    (:`  `
      (set `self.Secondaryammo` _result))))

(event `FireGun1`
  (bind _asprimary_gun (cast `PrimaryGun` (`ChildActorComponent.ChildActor` (`self.PrimaryWeapon`))))
  (`KismetSystemLibrary.Delay` 0.5)
  (`GunBase.Fire` _asprimary_gun))

(event `ReloadGun2`
  (bind _assecondarytestgun (cast `/Game/Blueprints/SECONDARYTESTGUN` (`ChildActorComponent.ChildActor` (`self.SecondaryWeapon`))))
  (`GunBase.Reload` _assecondarytestgun))

(event `self.AIPerception.OnPerceptionUpdated`
  (params (UpdatedActors :type "Array of Actor Object Reference (by ref)"))
  (for _array_element UpdatedActors
    (if (<= (`self.AIHealth`) 25)
      (cast `/Game/Blueprints/Health` _array_element)
      (`BlackboardComponent.SetValueAsObject` (`AIBlueprintHelperLibrary.GetBlackboard` (`AIBlueprintHelperLibrary.GetAIController` self)) "FoundPickup" _array_element)
      (`BlackboardComponent.SetValueAsBool` (`AIBlueprintHelperLibrary.GetBlackboard` (`AIBlueprintHelperLibrary.GetAIController` self)) "Fleeing" false)
      (`BlackboardComponent.SetValueAsBool` (`AIBlueprintHelperLibrary.GetBlackboard` (`AIBlueprintHelperLibrary.GetAIController` self)) "IsPickUpInReach?" true)
      (elif (== (`self.Secondaryammo`) 0)
        (cast `/Game/MyPickUpBase` _array_element)
        (`BlackboardComponent.SetValueAsBool` (`AIBlueprintHelperLibrary.GetBlackboard` (`AIBlueprintHelperLibrary.GetAIController` self)) "NeedAmmo" true)
        (`BlackboardComponent.SetValueAsObject` (`AIBlueprintHelperLibrary.GetBlackboard` (`AIBlueprintHelperLibrary.GetAIController` self)) "FoundPickup" _array_element)))))

(event `/Game/Blueprints/KillTrackerInterface.onKilledConfirmed`
  (params (KillerName :type String))
  (bind _asmy_game_instance (cast `/Game/MyGameInstance` (`GameplayStatics.GetGameInstance`)))
  (`/Game/MyGameInstance.AddPlayerData` _asmy_game_instance KillerName 0))

(fn `CheckPlayerVisbility`
  (bind _returnvalue (`GameplayStatics.GetActorOfClass` "/Game/Blueprints/MainCharacter.MainCharacter_C"))
  (`KismetSystemLibrary.LineTraceSingle` (`self.K2_GetActorLocation`) (`self.K2_GetActorLocation` _returnvalue) "TraceTypeQuery1"))

(fn `UserConstructionScript`)