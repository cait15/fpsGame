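; Health pickup actor that respawns after being touched by the player's MainCharacter or a BP_TheAI; no health is granted in this graph.
; It registers as a sight stimulus for AI perception and saves its starting scale.
; On overlap it shrinks to zero and disables cube collision, restoring both after a five-second delay.
; Only player pickups play the collect sound, guarded by a flag against repeats until respawn.
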(event `self.ReceiveBeginPlay`
  (set `self.pickupscale` (`self.GetActorScale3D`))
  (`AIPerceptionStimuliSourceComponent.RegisterForSense` (`self.AIPerceptionStimuliSource`) "/Script/AIModule.AISense_Sight"))

(event `self.ReceiveActorBeginOverlap`
  (params (OtherActor :type "Actor Object Reference"))
  (cast `/Game/Blueprints/MainCharacter` OtherActor
    (:`then`
      (if (not (`self.bool played sound`))
        (`GameplayStatics.PlaySound2D` "/Game/Audio/coin-collect-retro-8-bit-sound-effect-145251.coin-collect-retro-8-bit-sound-effect-145251" 1.0 1.0 0.0 null null)
        (set `self.bool played sound` true)
        (`self.SetActorScale3D` self (0.0 0.0 0.0) :!label _label)
        (`PrimitiveComponent.SetCollisionEnabled` (`self.Cube`) "NoCollision")
        (`KismetSystemLibrary.Delay` 5.0)
        (`self.SetActorScale3D` self (`self.pickupscale`))
        (`PrimitiveComponent.SetCollisionEnabled` (`self.Cube`) "QueryAndPhysics")
        (set `self.bool played sound` false)))
    (:`CastFailed`
      (cast `/Game/Blueprints/FixingAI/BP/BP_TheAI` OtherActor)
      (goto _label))))

(fn `UserConstructionScript`)